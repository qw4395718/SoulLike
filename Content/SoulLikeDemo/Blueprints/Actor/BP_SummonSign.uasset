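; BP_SummonSign is a summon sign actor for a souls-like demo, animated with two counter-rotating ring meshes.
; Each Tick calls the parent, then sets both rings' world yaw from game time times RotSpeed, negated for the second ring.
; The yaw is clamped to 0–360 rather than wrapped, so with a positive speed the spin stops after one turn of game time.
; The graph holds no overlap or summoning logic.
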(event `self.ReceiveTick`
  (params (DeltaSeconds :type "Float (single-precision)"))
  (bind _returnvalue (`KismetMathLibrary.MakeRotator` 0.0 0.0 (`KismetMathLibrary.FClamp` (* (`self.RotSpeed`) (`KismetSystemLibrary.GetGameTimeInSeconds`)) 0.0 360.0)))
  (`parent.ReceiveTick` 0.0)
  (`SceneComponent.K2_SetWorldRotation` (`self.RingMesh`) _returnvalue false false)
  (`SceneComponent.K2_SetWorldRotation` (`self.RingMesh2`) (* _returnvalue -1.0) false false))

(fn `UserConstructionScript`)