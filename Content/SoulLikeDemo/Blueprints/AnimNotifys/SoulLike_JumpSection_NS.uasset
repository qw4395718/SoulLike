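; Anim notify state that marks the combo window in montages or animations played by SoulLike_AnimMan_CharacterBP.
; On begin, it stores itself as the character's attack jump-section notify and sets EnableComboPeriod to true.
; On end, it clears that flag but leaves the stored notify reference in place.
; Both events do nothing further if the mesh owner is not that character class.
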(fn `Received_NotifyBegin`
  (params (MeshComp :type "SkeletalMeshComponent Object Reference") (Animation :type "AnimSequenceBase Object Reference") (TotalDuration :type "Float (double-precision)"))
  (returns (ReturnValue :type Boolean))
  (bind _assoul_like_anim_man_character_bp (cast `/Game/SoulLikeDemo/Blueprints/CharacterLogic/SoulLike_AnimMan_CharacterBP` (`ActorComponent.GetOwner` MeshComp)))
  (set `/Game/SoulLikeDemo/Blueprints/CharacterLogic/SoulLike_AnimMan_CharacterBP.SoulLikeAttackJumSectionNotify` self _assoul_like_anim_man_character_bp)
  (set `/Game/SoulLikeDemo/Blueprints/CharacterLogic/SoulLike_AnimMan_CharacterBP.bEnableComboPeriod` true _assoul_like_anim_man_character_bp)
  (return true))

(fn `Received_NotifyEnd`
  (params (MeshComp :type "SkeletalMeshComponent Object Reference") (Animation :type "AnimSequenceBase Object Reference"))
  (returns (ReturnValue :type Boolean))
  (bind _assoul_like_anim_man_character_bp (cast `/Game/SoulLikeDemo/Blueprints/CharacterLogic/SoulLike_AnimMan_CharacterBP` (`ActorComponent.GetOwner` MeshComp)))
  (set `/Game/SoulLikeDemo/Blueprints/CharacterLogic/SoulLike_AnimMan_CharacterBP.bEnableComboPeriod` false _assoul_like_anim_man_character_bp)
  (return false))